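; Drop zone actor that checks overlapping actors against an assigned target pickable object, accepting only the match.
; Colours from a parameter collection drive its dynamic material: yellow when idle, red briefly for wrong overlaps, green on success, each change with a sound.
; Success locks the zone, reports progress to the C_Congruent game mode, disables the target's physics and uses a timeline to lerp it onto the zone's location and rotation.
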(event Custom|Success
  (bind _targetobject (Variables|Default|GetTargetObject))
  (Utilities|FlowControl|Sequence
    (:then_0
      (bind _asc_congruent (Utilities|Casting|CastToC_Congruent (Game|GetGameMode)))
      (Default|UpdateProgress _asc_congruent))
    (:then_1
      (bind _returnvalue (Rendering|Material|GetVectorParameterValue "/Game/Itamar/Common/Materials/DropZone_Param.DropZone_Param" "Green" :!class /Script/Engine.KismetMaterialLibrary))
      (Rendering|Material|SetVectorParameterValue (Variables|Default|GetMat) "Colour" _returnvalue :!class /Script/Engine.MaterialInstanceDynamic)
      (Audio|PlaySoundatLocation "/Game/Itamar/Common/Sound/goat_baa_calm_03.goat_baa_calm_03" (Transformation|GetActorLocation) "0, 0, 0" 1.0 1.0 0.0 0 0 0 0))
    (:then_2
      (Physics|SetSimulatePhysics (Actor|GetComponentbyClass (Variables|Default|GetTargetObject) "/Script/Engine.PrimitiveComponent") false)
      (bind _newtrack_0 (Timeline|Timeline_0 Play)
        (:Update
          (Transformation|SetActorLocation _targetobject (Math|Vector|Lerp(Vector) (Transformation|GetActorLocation _targetobject) (Transformation|GetActorLocation) _newtrack_0) false false)
          (Transformation|SetActorRotation _targetobject (Math|Rotator|Lerp(Rotator) (Transformation|GetActorRotation _targetobject) (Transformation|GetActorRotation) _newtrack_0 true)))))))

(event Custom|Wrong
  (bind _returnvalue (Rendering|Material|GetVectorParameterValue "/Game/Itamar/Common/Materials/DropZone_Param.DropZone_Param" "Red" :!class /Script/Engine.KismetMaterialLibrary))
  (Rendering|Material|SetVectorParameterValue (Variables|Default|GetMat) "Colour" _returnvalue :!class /Script/Engine.MaterialInstanceDynamic)
  (Audio|PlaySoundatLocation "/Game/Itamar/Common/Sound/duck_quack_single_08.duck_quack_single_08" (Transformation|GetActorLocation) "0, 0, 0" 1.0 1.0 0.0 0 0 0 0)
  (Utilities|FlowControl|Delay 1.0)
  (CallFunction|ResetColour))

(event Custom|ResetColour
  (bind _returnvalue (Rendering|Material|GetVectorParameterValue "/Game/Itamar/Common/Materials/DropZone_Param.DropZone_Param" "Yellow" :!class /Script/Engine.KismetMaterialLibrary))
  (Rendering|Material|SetVectorParameterValue (Variables|Default|GetMat) "Colour" _returnvalue :!class /Script/Engine.MaterialInstanceDynamic)
  (Audio|PlaySoundatLocation "/Game/Itamar/Common/Sound/ui_button_simple_click_01.ui_button_simple_click_01" (Transformation|GetActorLocation) "0, 0, 0" 1.0 1.0 0.2 0 0 0 0))

(event Collision|EventActorBeginOverlap
  (params (OtherActor :type Actor%20Object%20Reference))
  (if (not (Variables|Default|GetFinished))
    (bind _targetobject (Variables|Default|GetTargetObject)
      (:then
        (Utilities|IsValid (Actor|GetComponentbyClass OtherActor "/Game/Itamar/Common/Blueprints/Pickable.Pickable_C")
          (:Is%20Valid
            (if (== OtherActor _targetobject)
              (Variables|Default|SetFinished true)
              (CallFunction|Success)
              (else
                (CallFunction|Wrong :!label _label))))
          (:Is%20Not%20Valid
            (goto _label))))
      (:else))))

(event Collision|EventActorEndOverlap
  (params (OtherActor :type Actor%20Object%20Reference)))

(fn ConstructionScript
  (bind _staticmeshcomponent (Variables|Debug|GetStaticMeshComponent))
  (bind _returnvalue (Rendering|Material|CreateDynamicMaterialInstance _staticmeshcomponent 0 "/Game/Itamar/Common/Materials/DropZone.DropZone" "None" :!class /Script/Engine.PrimitiveComponent))
  (bind _output_get (Variables|Default|SetMat _returnvalue))
  (Rendering|Material|SetMaterial _staticmeshcomponent 0 _output_get)
  (bind _returnvalue_2 (Rendering|Material|GetVectorParameterValue "/Game/Itamar/Common/Materials/DropZone_Param.DropZone_Param" "Yellow" :!class /Script/Engine.KismetMaterialLibrary))
  (Rendering|Material|SetVectorParameterValue _output_get "Colour" _returnvalue_2 :!class /Script/Engine.MaterialInstanceDynamic))