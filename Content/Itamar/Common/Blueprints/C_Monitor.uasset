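; An in-world monitor actor that cycles pictures on its screen and shows game progress on a widget UI.
; On BeginPlay it binds the widget's button to step through the Pictures array, wrapping at the end, via a texture parameter on a dynamic material instance.
; Init_Event subscribes to the C_Congruent game mode's update, which feeds drop zone counts and game time percent (as a battery bar) into the widget.
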(event Custom|NextPicture
  (bind _pictures (Variables|Default|GetPictures))
  ;[1 1 1] Setting new image
  (bind _output_get (Variables|Default|SetcurrentIndex (+ (Variables|Default|GetcurrentIndex) 1)))
  (if (>= _output_get (Utilities|Array|Length _pictures))
    (Variables|Default|SetcurrentIndex 0))
  (Variables|/Game/Itamar/Common/Blueprints/C_MonitorWidget.C_MonitorWidget_C|SetcurrentIndex (Variables|Default|GetMonitorInstance) (+ (Variables|Default|GetcurrentIndex) 1))
  (Rendering|Material|SetTextureParameterValue (Variables|Default|GetMat) "Texture" (Utilities|Array|Get(acopy) _pictures (Variables|Default|GetcurrentIndex))))

(event Custom|Init_Event
  (bind _asc_congruent (Utilities|Casting|CastToC_Congruent (Game|GetGameMode)))
  (Variables|Default|SetGameMode true)
  (EventDispatchers|BindEventtoUpdateData _asc_congruent (delegate Custom|UpdateData)))

(event Custom|OnPressedUIButton
  ;[1 1 1] Binding the event from the Widger (UI)
  (CallFunction|NextPicture))

(event Custom|UpdateData
  (bind _monitorinstance (Variables|Default|GetMonitorInstance))
  (Utilities|FlowControl|Sequence
    (:then_0
      (Variables|/Game/Itamar/Common/Blueprints/C_MonitorWidget.C_MonitorWidget_C|SetTotalDropzones _monitorinstance (Variables|/Game/Itamar/Common/Blueprints/C_Congruent.C_Congruent_C|GetDropZonesNum (stale Custom|Init_Event _asc_congruent)))
      (Variables|/Game/Itamar/Common/Blueprints/C_MonitorWidget.C_MonitorWidget_C|SetFinishedDropzones _monitorinstance (Variables|/Game/Itamar/Common/Blueprints/C_Congruent.C_Congruent_C|GetDropZonesNumReady (stale Custom|Init_Event _asc_congruent))))
    (:then_1
      (Progress|SetPercent (Variables|/Game/Itamar/Common/Blueprints/C_MonitorWidget.C_MonitorWidget_C|GetBattery_ProgressBar (Variables|Default|GetMonitorInstance)) (Variables|/Game/Itamar/Common/Blueprints/C_Congruent.C_Congruent_C|GetGameTimePercent (stale Custom|Init_Event _asc_congruent))))))

(event EventBeginPlay
  (bind _monitorscreen (Variables|Default|GetMonitorScreen))
  ;[1 1 1] Binding the event from the Widger (UI)
  (bind _asc_monitor_widget (Utilities|Casting|CastToC_MonitorWidget (UserInterface|GetWidget (Variables|Default|GetMonitorUI)))
    (:then
      (Variables|Default|SetMonitorInstance _asc_monitor_widget)
      (EventDispatchers|AssignOnPressed (Variables|/Game/Itamar/Common/Blueprints/C_MonitorWidget.C_MonitorWidget_C|GetButton_237 _asc_monitor_widget) (delegate Custom|OnPressedUIButton))
      ;[1 1 1] Making a new Material Instance
      (bind _returnvalue (Rendering|Material|CreateDynamicMaterialInstance _monitorscreen 0 "/Game/Itamar/Common/Materials/MonitorScreenMat.MonitorScreenMat" "None" :!class /Script/Engine.PrimitiveComponent))
      (bind _output_get (Variables|Default|SetMat _returnvalue))
      (Rendering|Material|SetMaterial _monitorscreen 0 _output_get)
      (Variables|/Game/Itamar/Common/Blueprints/C_MonitorWidget.C_MonitorWidget_C|SettotalIndex (Variables|Default|GetMonitorInstance) (Utilities|Array|Length (Variables|Default|GetPictures)))
      ;[1 1 1] Setting new image
      (Variables|Default|SetcurrentIndex 0)
      (Variables|/Game/Itamar/Common/Blueprints/C_MonitorWidget.C_MonitorWidget_C|SetcurrentIndex (Variables|Default|GetMonitorInstance) (+ (Variables|Default|GetcurrentIndex) 1))
      (Rendering|Material|SetTextureParameterValue (Variables|Default|GetMat) "Texture" (Utilities|Array|Get(acopy) (Variables|Default|GetPictures) (Variables|Default|GetcurrentIndex))))
    (:CastFailed
      (Development|PrintString "Something went wrong, itamar."))))

(fn ConstructionScript)