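; C_Congruent runs the rules for a timed drop-zone game, apparently as its game mode, tracking a countdown and completion progress.
; BeginPlay counts the drop zones, starts a looping timer, initializes every monitor and broadcasts initialization.
; Each timer update lowers the remaining time and broadcasts data, with no stop at zero.
; UpdateProgress counts ready zones, broadcasts changes and only prints "GameEnded" when all are ready.
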(event Custom|UpdateProgress
  (bind _output_get (Variables|Default|SetDropZonesNumReady (+ (Variables|Default|GetDropZonesNumReady) 1)))
  (Default|CallProgressChanged)
  (if (>= _output_get (Variables|Default|GetDropZonesNum))
    (Development|PrintString "GameEnded")))

(event Custom|UpdateTimer
  (bind _output_get (Variables|Default|SetCurrentTime (- (Variables|Default|GetCurrentTime) (Variables|Default|GetTimerInterval))))
  (Variables|Default|SetGameTimePercent (Math|Float|SafeDivide (Math|Conversions|ToFloat(Integer) _output_get) (Math|Conversions|ToFloat(Integer) (Variables|Default|GetTotalTime))))
  (Default|CallUpdateData))

(event EventBeginPlay
  (bind _timerinterval (Variables|Default|GetTimerInterval))
  (Utilities|FlowControl|Sequence
    (:then_0
      (bind _outactors (Actor|GetAllActorsOfClass "/Game/Itamar/Common/Blueprints/C_ObjectDropZone.C_ObjectDropZone_C"))
      (bind _output_get (Variables|Default|SetDropzonesInstances _outactors))
      (Variables|Default|SetDropZonesNum (Utilities|Array|Length _output_get))
      (Variables|Default|SetDropZonesNumReady 0))
    (:then_1
      (Variables|Default|SetCurrentTime (Variables|Default|GetTotalTime))
      (Utilities|Time|SetTimerbyEvent (delegate Custom|UpdateTimer) (Math|Conversions|ToFloat(Integer) _timerinterval) true)
      (bind _output_get_2 (Variables|Default|SetCurrentTime (- (Variables|Default|GetCurrentTime) _timerinterval)))
      (Variables|Default|SetGameTimePercent (Math|Float|SafeDivide (Math|Conversions|ToFloat(Integer) _output_get_2) (Math|Conversions|ToFloat(Integer) (Variables|Default|GetTotalTime))))
      (Default|CallUpdateData))
    (:then_2
      (bind _outactors_2 (Actor|GetAllActorsOfClass "/Game/Itamar/Common/Blueprints/C_Monitor.C_Monitor_C"))
      (for _array_element _outactors_2
        (Default|InitEvent _array_element)))
    (:then_3
      (Default|CallGameModeInititalized))))

(fn ConstructionScript)